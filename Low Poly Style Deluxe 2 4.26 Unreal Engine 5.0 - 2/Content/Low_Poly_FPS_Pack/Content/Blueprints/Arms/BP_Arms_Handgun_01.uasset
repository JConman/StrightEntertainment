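; First-person handgun arms character with a grappling hook for swinging through the level.
; Left click sphere-traces from the Slider along camera forward, saves the impact point and attaches the visible Cable to a spawned HookPoint actor.
; While attached, Tick applies a dot-product tether force against velocity along the rope axis, plus a constant push along camera forward.
; Right click or landing clears the grapple and hides the Cable, without destroying the spawned actor.
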(event `Key|LeftMouseButton`
  (params (Key :type "Key Structure"))
  (bind _cable (`self.Cable`))
  (bind _returnvalue (`SceneComponent.K2_GetComponentLocation` (`self.Slider`)))
  (:`Pressed`
    (bind (_outhit _returnvalue_2) (`KismetSystemLibrary.SphereTraceSingle` :`Start` _returnvalue :`End` (+ (* (`self.GetActorForwardVector` (`GameplayStatics.GetPlayerCameraManager` 0)) (`self.Hook Length`)) _returnvalue) :`Radius` 15.0 :`TraceChannel` "TraceTypeQuery1" :`DrawDebugType` "ForDuration"))
    (if _returnvalue_2
      (bind _output_get (set `self.hook Point` (`.ImpactPoint` (`GameplayStatics.BreakHitResult` _outhit))))
      (set `self.Grapple Attached` true)
      (`SceneComponent.SetHiddenInGame` _cable false false)
      (bind _returnvalue_3 (`|SpawnActorFromClass` "/Game/Low_Poly_FPS_Pack/Content/Blueprints/HookPoint.HookPoint_C" (`KismetMathLibrary.MakeTransform` _output_get) "Undefined" "OverrideRootScale" null null))
      (`CableComponent.SetAttachEndTo` _cable _returnvalue_3 "None" "None"))))

(event `Key|RightMouseButton`
  (params (Key :type "Key Structure"))
  (:`Pressed`
    (set `self.Grapple Attached` false :!label _label)
    (`SceneComponent.SetHiddenInGame` (`self.Cable`) true false)))

(event `self.OnLanded`
  (params (Hit :type "HitResult Structure (by ref)"))
  (goto _label))

(event `self.ReceiveTick`
  (params (DeltaSeconds :type "Float (single-precision)"))
  (bind _returnvalue (- (`self.K2_GetActorLocation`) (`self.Hook Point`)))
  (if (`self.Grapple Attached`)
    (`CharacterMovementComponent.AddForce` (`self.CharacterMovement`) (* (* (`KismetMathLibrary.Dot_VectorVector` (`self.GetVelocity`) _returnvalue) (`KismetMathLibrary.Normal` _returnvalue)) -3.0))
    (`CharacterMovementComponent.AddForce` (`self.CharacterMovement`) (* (`self.GetActorForwardVector` (`GameplayStatics.GetPlayerCameraManager` 0)) 50000.0))))

(fn `UserConstructionScript`)